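; BP_RoomSpawner is a procedural level generator node that loads a room as a level instance on a grid, then destroys itself.
; On BeginPlay it registers with MainGameInstance unless an upward trace hits existing geometry.
; SpawnRoom picks room shape and rotation from free neighbouring cells using the seed, then chains to the next spawner, passing taken locations.
; At zero count, random spawners place boss, shop, treasure and endcap rooms; level choice within each pool is unseeded.
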(event `self.ReceiveBeginPlay`
  (bind (_returnvalue_x _returnvalue_y) (`KismetMathLibrary.BreakVector` (`SceneComponent.K2_GetComponentLocation` (`self.DefaultSceneRoot`))))
  (bind _returnvalue (`SceneComponent.K2_GetComponentLocation` (`self.RaycastSource`)))
  (bind _levelgridresolution (`/Game/FirstPersonBP/Blueprints/MainGameInstance.LevelGridResolution` (`self.GameInstanceRef`)))
  ;[1 0.2344 0] If the spawner is placed in place of some already existing level, just destroy it
  (bind (_outhit _returnvalue_2) (`KismetSystemLibrary.LineTraceSingle` _returnvalue (`KismetMathLibrary.MakeVector` (.x _returnvalue) (.y _returnvalue) (+ (.z _returnvalue) 1000.0)) "TraceTypeQuery1"))
  (`KismetSystemLibrary.PrintString` (`KismetStringLibrary.Conv_BoolToString` _returnvalue_2) true true (struct :`R` 1.0 :`B` 0.543339 :`A` 1.0))
  (if _returnvalue_2
    (`self.K2_DestroyActor`)
    (else
      (bind _asmain_game_instance (cast `/Game/FirstPersonBP/Blueprints/MainGameInstance` (`GameplayStatics.GetGameInstance`)))
      (bind _output_get (set `self.GameInstanceRef` _asmain_game_instance))
      ;[0 0.625 1] Add reference to self to a list of active spawners
      (`KismetArrayLibrary.Array_Add` (`/Game/FirstPersonBP/Blueprints/MainGameInstance.ActiveSpawners` _output_get) self)
      (set `self.SelfLocation` (make `/Game/FirstPersonBP/IntVector2D` (`KismetMathLibrary.Round` (`KismetMathLibrary.GridSnap_Float` _returnvalue_x _levelgridresolution)) (`KismetMathLibrary.Round` (`KismetMathLibrary.GridSnap_Float` _returnvalue_y _levelgridresolution)))))))

(event `SpawnRoom`
  (params (LevelCounter :type Integer) (TakenLocations :type "Array of /Game/FirstPersonBP/IntVector2D Structure"))
  (bind _gameinstanceref (`self.GameInstanceRef`))
  (bind _takenlocations (`self.TakenLocations`))
  (bind _gameinstanceref_2 (`self.GameInstanceRef`))
  (bind _defaultsceneroot (`self.DefaultSceneRoot`))
  (bind _gameinstanceref_3 (`self.GameInstanceRef`))
  (bind _seed (`/Game/FirstPersonBP/Blueprints/MainGameInstance.Seed` _gameinstanceref_2))
  (bind _seed_2 (`/Game/FirstPersonBP/Blueprints/MainGameInstance.Seed` (`self.GameInstanceRef`)))
  (bind (_left _left__2 _right _right__2 _forward _forward__2) (`/Game/Library/MyMacroLibrary.GetLocations` (`SceneComponent.GetForwardVector` _defaultsceneroot) (`SceneComponent.GetRightVector` _defaultsceneroot) (`/Game/FirstPersonBP/Blueprints/MainGameInstance.LevelGridResolution` _gameinstanceref) (`self.SelfLocation`)))
  (bind _output_get (set `self.LevelNumberLimit` LevelCounter))
  (`KismetSystemLibrary.PrintString` (`KismetStringLibrary.Conv_IntToString` _output_get))
  (set `self.TakenLocations` TakenLocations)
  ;[0 0.5547 1] Check counter
  (if (<= LevelCounter 0)
    (`self.Spawn Boss` (`/Game/Library/MyMacroLibrary.GetRandom (seeded)` (`/Game/FirstPersonBP/Blueprints/MainGameInstance.ActiveSpawners` _gameinstanceref_3) (`/Game/FirstPersonBP/Blueprints/MainGameInstance.Seed` _gameinstanceref_3)) (`self.TakenLocations`))
    (`self.K2_DestroyActor`)
    (else
      ;[0.6875 1 0] Check doubled spawner
      (if (== (`KismetArrayLibrary.Array_Find` (`self.TakenLocations`) (`self.SelfLocation`)) -1)
        ;[1 0.5391 0] Add location to list of taken locations
        (`self.AddSelfToTakenLocations`)
        ;[1 0 0.7734] Remove spawner from list of available spawners
        (`KismetArrayLibrary.Array_RemoveItem` (`/Game/FirstPersonBP/Blueprints/MainGameInstance.ActiveSpawners` _gameinstanceref) self)
        ;[0.4297 1 0] Check free directions
        (`self.CheckCombinations` (not (and (== (`KismetArrayLibrary.Array_Find` _takenlocations _left) -1) (== (`KismetArrayLibrary.Array_Find` _takenlocations _left__2) -1))) (not (and (== (`KismetArrayLibrary.Array_Find` _takenlocations _right) -1) (== (`KismetArrayLibrary.Array_Find` _takenlocations _right__2) -1))) (not (and (== (`KismetArrayLibrary.Array_Find` _takenlocations _forward) -1) (== (`KismetArrayLibrary.Array_Find` _takenlocations _forward__2) -1)))
          (:`LeftRightFront`
            ;[1 0.4922 0] Sets possible rotations a room can have and randomize room type
            (switch `int` (`KismetMathLibrary.RandomIntegerInRangeFromStream` 0 3 _seed_2)
              (:`0`
                ;[0 1 0.6953] Spawn room
                (bind _boutsuccess (`self.CustomSpawnRoom` (`/Game/FirstPersonBP/Blueprints/MainGameInstance.Crosses` _gameinstanceref_2) (`KismetMathLibrary.RandomIntegerInRangeFromStream` 0 3 _seed))
                  (:`exec2`
                    (`KismetSystemLibrary.PrintString` (`KismetStringLibrary.Conv_BoolToString` _boutsuccess)))))
              (:`1`
                (set `self.MinRot` -1)
                (set `self.MaxRot` 1)
                (bind _boutsuccess_2 (`self.CustomSpawnRoom` (`/Game/FirstPersonBP/Blueprints/MainGameInstance.Threeways` _gameinstanceref_2) (`KismetMathLibrary.RandomIntegerInRangeFromStream` (`self.MinRot`) (`self.MaxRot`) _seed) :!label _label)
                  (:`exec2`
                    (`KismetSystemLibrary.PrintString` (`KismetStringLibrary.Conv_BoolToString` _boutsuccess_2)))))
              (:`2`
                (set `self.MinRot` 0)
                (set `self.MaxRot` 1)
                (bind _boutsuccess_3 (`self.CustomSpawnRoom` (`/Game/FirstPersonBP/Blueprints/MainGameInstance.Corners` _gameinstanceref_2) (`KismetMathLibrary.RandomIntegerInRangeFromStream` (`self.MinRot`) (`self.MaxRot`) _seed) :!label _label_2)
                  (:`exec2`
                    (`KismetSystemLibrary.PrintString` (`KismetStringLibrary.Conv_BoolToString` _boutsuccess_3)))))
              (:`3`
                (bind _boutsuccess_4 (`self.CustomSpawnRoom` (`/Game/FirstPersonBP/Blueprints/MainGameInstance.Corridors` _gameinstanceref_2) (* (`KismetMathLibrary.RandomIntegerInRangeFromStream` 0 1 _seed) 2) :!label _label_3)
                  (:`exec2`
                    (`KismetSystemLibrary.PrintString` (`KismetStringLibrary.Conv_BoolToString` _boutsuccess_4)))))))
          (:`RightFront`
            (switch `int` (`KismetMathLibrary.RandomIntegerInRangeFromStream` 0 2 _seed_2)
              (:`0`
                (set `self.MinRot` -1)
                (set `self.MaxRot` -1)
                (goto _label))
              (:`1`
                (set `self.MinRot` 0)
                (set `self.MaxRot` 0)
                (goto _label_2))
              (:`2`
                (goto _label_3))))
          (:`LeftFront`
            (switch `int` (`KismetMathLibrary.RandomIntegerInRangeFromStream` 0 2 _seed_2)
              (:`0`
                (set `self.MinRot` 1)
                (set `self.MaxRot` 1)
                (goto _label))
              (:`1`
                (set `self.MinRot` 1)
                (set `self.MaxRot` 1)
                (goto _label_2))
              (:`2`
                (goto _label_3))))
          (:`LeftRight`
            (switch `int` (`KismetMathLibrary.RandomIntegerInRangeFromStream` 0 2 _seed_2)
              (:`0`
                (set `self.MinRot` 0)
                (set `self.MaxRot` 0)
                (goto _label))
              (:`1`
                (set `self.MinRot` 0)
                (set `self.MaxRot` 1)
                (goto _label_2))))
          (:`Left  `
            (set `self.MinRot` 1)
            (set `self.MaxRot` 1)
            (goto _label_2))
          (:`Right `
            (set `self.MinRot` 0)
            (set `self.MaxRot` 0)
            (goto _label_2))
          (:`Front `
            (goto _label_3))
          (:`None `
            (bind _boutsuccess_5 (`self.CustomSpawnRoom` (`/Game/FirstPersonBP/Blueprints/MainGameInstance.Endcaps` _gameinstanceref_2))
              (:`exec2`
                (`KismetSystemLibrary.PrintString` (`KismetStringLibrary.Conv_BoolToString` _boutsuccess_5))))))
        (`self.SpawnNext`)
        (else
          (`KismetArrayLibrary.Array_RemoveItem` (`/Game/FirstPersonBP/Blueprints/MainGameInstance.ActiveSpawners` (`self.GameInstanceRef`)) self)
          (`self.SpawnNext`))))))

(event `SpawnNext`
  (bind _output (`|GetArrayItem` (`/Game/FirstPersonBP/Blueprints/MainGameInstance.ActiveSpawners` (`self.GameInstanceRef`))))
  ;[1 0.4453 0] Spawn next room
  ;;[1 0 0] ¯\_(ツ)_/¯
  (`KismetSystemLibrary.Delay` 0.2) ; No clue why, but doesn't work without this delay
  (`/Engine/EditorBlueprintResources/StandardMacros.IsValid` _output
    (:`Is Valid`
      (`self.SpawnRoom` _output (- (`self.LevelNumberLimit`) 1) (`self.TakenLocations`))
      (`self.K2_DestroyActor`))
    (:`Is Not Valid`
      (`KismetSystemLibrary.PrintString` "Invalid Room" true true (struct :`R` 1.0 :`A` 1.0) 60.0))))

(event `Spawn Boss`
  (params (TakenLocations :type "Array of /Game/FirstPersonBP/IntVector2D Structure"))
  (bind _gameinstanceref (`self.GameInstanceRef`))
  (bind _output (`/Game/Library/MyMacroLibrary.GetRandom (seeded)` (`/Game/FirstPersonBP/Blueprints/MainGameInstance.ActiveSpawners` _gameinstanceref) (`/Game/FirstPersonBP/Blueprints/MainGameInstance.Seed` _gameinstanceref)))
  ;[1 0 0.9609] Try to spawn a boss room
  (bind _output_get (set `self.TakenLocations` TakenLocations))
  (if (== (`KismetArrayLibrary.Array_Find` _output_get (`self.SelfLocation`)) -1)
    (`self.CustomSpawnRoom` (`/Game/FirstPersonBP/Blueprints/MainGameInstance.Bossrooms` _gameinstanceref)
      (:`exec2`
        (`self.RemoveSelf`)
        (`self.AddSelfToTakenLocations`)
        (`self.Spawn Shop` _output (`self.TakenLocations`))
        (`self.K2_DestroyActor` :!label _label_4)))
    (else
      (`self.RemoveSelf`)
      (`self.Spawn Boss` _output (`self.TakenLocations`))
      (`self.K2_DestroyActor`))))

(event `Spawn Shop`
  (params (TakenLocations :type "Array of /Game/FirstPersonBP/IntVector2D Structure"))
  (bind _gameinstanceref (`self.GameInstanceRef`))
  (bind _output (`/Game/Library/MyMacroLibrary.GetRandom (seeded)` (`/Game/FirstPersonBP/Blueprints/MainGameInstance.ActiveSpawners` _gameinstanceref) (`/Game/FirstPersonBP/Blueprints/MainGameInstance.Seed` _gameinstanceref)))
  ;[1 0 0.6094] Try to spawn a shop
  (bind _output_get (set `self.TakenLocations` TakenLocations))
  (if (== (`KismetArrayLibrary.Array_Find` _output_get (`self.SelfLocation`)) -1)
    (`self.CustomSpawnRoom` (`/Game/FirstPersonBP/Blueprints/MainGameInstance.Shops` _gameinstanceref)
      (:`exec2`
        (`self.RemoveSelf`)
        (`self.AddSelfToTakenLocations`)
        (`self.Spawn Treasure` _output (`self.TakenLocations`))
        (goto _label_4)))
    (else
      (`self.RemoveSelf`)
      (`self.Spawn Shop` _output (`self.TakenLocations`))
      (`self.K2_DestroyActor`))))

(event `Spawn Treasure`
  (params (TakenLocations :type "Array of /Game/FirstPersonBP/IntVector2D Structure"))
  (bind _gameinstanceref (`self.GameInstanceRef`))
  (bind _output (`/Game/Library/MyMacroLibrary.GetRandom (seeded)` (`/Game/FirstPersonBP/Blueprints/MainGameInstance.ActiveSpawners` _gameinstanceref) (`/Game/FirstPersonBP/Blueprints/MainGameInstance.Seed` _gameinstanceref)))
  ;[1 0 0.1875] Try to spawn a treasure room
  (bind _output_get (set `self.TakenLocations` TakenLocations))
  (if (== (`KismetArrayLibrary.Array_Find` _output_get (`self.SelfLocation`)) -1)
    (`self.CustomSpawnRoom` (`/Game/FirstPersonBP/Blueprints/MainGameInstance.TreasureRooms` _gameinstanceref)
      (:`exec2`
        (`self.RemoveSelf`)
        (`self.AddSelfToTakenLocations`)
        (`self.SpawnEndcap` _output (`self.TakenLocations`))
        (goto _label_4)))
    (else
      (`self.RemoveSelf`)
      (`self.Spawn Treasure` _output (`self.TakenLocations`))
      (`self.K2_DestroyActor`))))

(event `SpawnEndcap`
  (params (TakenLocations :type "Array of /Game/FirstPersonBP/IntVector2D Structure"))
  (bind _gameinstanceref (`self.GameInstanceRef`))
  (bind _activespawners (`/Game/FirstPersonBP/Blueprints/MainGameInstance.ActiveSpawners` _gameinstanceref))
  (bind _output (`/Game/Library/MyMacroLibrary.GetRandom (seeded)` _activespawners (`/Game/FirstPersonBP/Blueprints/MainGameInstance.Seed` _gameinstanceref)))
  ;[0.6616 0.1042 1] Try to spawn an endcap
  (bind _output_get (set `self.TakenLocations` TakenLocations))
  (if (> (`KismetArrayLibrary.Array_Length` _activespawners) 0)
    (if (== (`KismetArrayLibrary.Array_Find` _output_get (`self.SelfLocation`)) -1)
      (`self.CustomSpawnRoom` (`/Game/FirstPersonBP/Blueprints/MainGameInstance.Endcaps` _gameinstanceref)
        (:`exec2`
          (`self.RemoveSelf`)
          (`self.AddSelfToTakenLocations`)
          (`self.SpawnEndcap` _output (`self.TakenLocations`))
          (goto _label_4)))
      (else
        (`self.RemoveSelf`)
        (`/Engine/EditorBlueprintResources/StandardMacros.IsValid` _output
          (:`Is Valid`
            (`self.SpawnEndcap` _output (`self.TakenLocations`)))
          (:`Is Not Valid`
            (`self.RemoveSelf`)))
        (`self.K2_DestroyActor`)))
    (else
      (`self.RemoveSelf`)
      (`self.K2_DestroyActor`))))

(fn `UserConstructionScript`)